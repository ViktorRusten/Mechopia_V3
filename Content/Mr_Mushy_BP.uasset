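; Mr Mushy is an enemy in Mechopia that chases the player and triggers damage on contact.
; Every Tick it uses SimpleMoveToActor through its instigator controller to follow the player character.
; When overlapping the player, it casts to MechopiaCharacter, calls DealDamage, then stores and prints the returned value.
; The player reference cached on BeginPlay is unused here, and the overlap branch has a hard-coded true condition.
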(event Collision|EventActorBeginOverlap
  (params (OtherActor :type Actor%20Object%20Reference))
  (bind _returnvalue (Game|GetPlayerCharacter 0))
  (if (Collision|IsOverlappingActor _returnvalue :!class /Script/Engine.Actor)
    (if true
      (Utilities|Casting|CastToMechopiaCharacter _returnvalue)
      (bind _output_get (Variables|Default|SetNewVar_0 (Class|MrMushy|DealDamage self)))
      (Development|PrintText (Utilities|Text|ToText(Integer) _output_get)))))

(event EventTick
  (params (DeltaSeconds :type Float%20%28single-precision%29))
  (bind _returnvalue (Game|GetPlayerCharacter 0))
  (Utilities|IsValid _returnvalue
    (:Is%20Valid
      (AI|Navigation|SimpleMovetoActor (Game|GetInstigatorController) _returnvalue))))

(event EventBeginPlay
  (Variables|Default|SetThePlayerActor (Game|GetPlayerCharacter 0)))

(fn ConstructionScript)